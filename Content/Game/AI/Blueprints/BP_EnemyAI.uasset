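; Enemy AI pawn that chases the player, attacks and dies when damage depletes its health.
; PawnSensing sightings set a seen flag and start AIMoveTo toward the player, with a cooldown-gated attack montage (not yet assigned) on arrival.
; Each chase also restarts a retriggerable delay that sends it to a random nearby navigable point once sightings stop.
; Tick prints the sight flag as a debug test; the flag never effectively clears.
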(event `self.ReceiveTick`
  (params (DeltaSeconds :type "Float (single-precision)"))
  ; testing for if the sight thingy works
  (if (`self.IsSeeingMouse`)
    (`KismetSystemLibrary.PrintString` "I Can See YOU")
    (`KismetSystemLibrary.Delay` 1.0)
    (else
      (`KismetSystemLibrary.PrintString` "no longer see anyone :(")
      (`KismetSystemLibrary.Delay` 1.0))))

(event `self.PawnSensing.OnSeePawn`
  (params (Pawn :type "Pawn Object Reference"))
  (set `self.IsSeeingMouse` true)
  (`self.FollowPlayer`))

(event `FollowPlayer`
  (if (`self.IsSeeingMouse`)
    (`|AIMoveTo` self (0.0 0.0 0.0) (`GameplayStatics.GetPlayerCharacter` 0) 50.0
      (:`then`
        (`KismetSystemLibrary.RetriggerableDelay` 2.0)
        (`self.MoveToRandomLocation`))
      (:`OnSuccess`
        (if (`self.CanAttack`)
          (set `self.CanAttack` false)
          ; need to set animation montage of attack
          (bind _returnvalue (`self.PlayAnimMontage` null))
          (`KismetSystemLibrary.Delay` _returnvalue)
          (set `self.CanAttack` true))))
    (else
      (set `self.IsSeeingMouse` false))))

(event `MoveToRandomLocation`
  (bind _randomlocation (`NavigationSystemV1.K2_GetRandomLocationInNavigableRadius` (`self.K2_GetActorLocation`) 500.0 null null))
  (`|AIMoveTo` self _randomlocation null))

(event `self.ReceiveAnyDamage`
  (params (Damage :type "Float (single-precision)") (DamageType :type "DamageType Object Reference") (InstigatedBy :type "Controller Object Reference") (DamageCauser :type "Actor Object Reference"))
  ; Damage
  (bind _output_get (set `self.Health` (- (`self.Health`) Damage)))
  ;; Check to see if health is below 0
  (if (<= _output_get 0.0)
    (`self.K2_DestroyActor`)))

(fn `UserConstructionScript`)