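; BP_Ammo is a weapon projectile actor that damages tagged actors it overlaps.
; On overlap it ignores its owner, checks the other actor's tags against DamagedActorTag, and on a match applies Damage and destroys itself.
; The construction script feeds Speed into the projectile movement's initial speed and uses Lifespan to limit how long the actor lives.
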(event `self.ReceiveActorBeginOverlap`
  (params (OtherActor :type "Actor Object Reference"))
  ; Damage
  (if (!= OtherActor (`self.GetOwner`))
    (for _array_element (`Actor.Tags` OtherActor)
      (if (== _array_element (`self.DamagedActorTag`))
        (`GameplayStatics.ApplyDamage` OtherActor (`self.Damage`))
        (`self.K2_DestroyActor`)))))

(fn `UserConstructionScript`
  (`parent.UserConstructionScript`)
  (set `ProjectileMovementComponent.InitialSpeed` (`self.Speed`) (`self.ProjectileMovement`))
  (`self.SetLifeSpan` (`self.Lifespan`)))