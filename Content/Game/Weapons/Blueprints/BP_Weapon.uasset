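; Base weapon actor that takes its mesh, fire type, ammo class, fire rate and emission socket from WeaponData.
; Activate and deactivate events toggle visibility, collision and tick, with deactivation also stopping fire.
; Start fire branches on single or automatic mode, the latter running a looping timer that spawns ammo at the mesh socket.
; Stop fire clears that timer.
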(event `self.ReceiveBeginPlay`
  (bind (_name _mesh) (break `/Game/Game/Weapons/Data/F_WeaponData` (`self.WeaponData`)))
  ; SetMesh
  (`/Engine/EditorBlueprintResources/StandardMacros.IsValid` _mesh
    (:`Is Valid`
      (`StaticMeshComponent.SetStaticMesh` (`self.StaticMesh`) _mesh))))

(event `OnActivate`
  ; Activate
  (`self.SetActorHiddenInGame` false)
  (`self.SetActorEnableCollision` true)
  (`self.SetActorTickEnabled` true))

(event `OnDeactivate`
  ; Deactivate
  (`self.SetActorHiddenInGame` true)
  (`self.SetActorEnableCollision` false)
  (`self.SetActorTickEnabled` false)
  (`self.OnStopFire`))

(event `OnStartFire`
  (bind (_weapondata_name _weapondata_mesh _weapondata_mountsocket _weapondata_emissionsocket _weapondata_weaponclass _weapondata_ammoclass _weapondata_ammofiretype _weapondata_ammofirerate) (break `/Game/Game/Weapons/Data/F_WeaponData` (`self.WeaponData`)))
  ; WeaponFiring
  (switch `/Game/Game/Weapons/Data/E_FireType` _weapondata_ammofiretype
    (:`NewEnumerator1`
      (`self.OnFire`))
    (:`NewEnumerator3`
      (bind _returnvalue (`KismetSystemLibrary.K2_SetTimerDelegate` (delegate `OnFire`) _weapondata_ammofirerate true))
      (set `self.FireTimer` _returnvalue))))

(event `OnFire`
  (bind (_weapondata_name _weapondata_mesh _weapondata_mountsocket _weapondata_emissionsocket _weapondata_weaponclass _weapondata_ammoclass _weapondata_ammofiretype _weapondata_ammofirerate) (break `/Game/Game/Weapons/Data/F_WeaponData` (`self.WeaponData`)))
  ; WeaponFiring
  (`|SpawnActorFromClass` _weapondata_ammoclass (`SceneComponent.GetSocketTransform` (`self.StaticMesh`) _weapondata_emissionsocket "RTS_World") "Undefined" "MultiplyWithRoot" (`self.GetOwner`) null))

(event `OnStopFire`
  ; StopFire
  (`KismetSystemLibrary.K2_ClearAndInvalidateTimerHandle` (`self.FireTimer`)))

(fn `UserConstructionScript`)