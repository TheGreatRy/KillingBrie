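; BP_Functions is a set of general math helpers for directions, aim points and offsets.
; SignedAngle takes the arccosine of two vectors' dot product and signs it by their cross product's Z.
; GetForwardAimLocation projects a point a given distance along a follower actor's forward vector.
; SignByPosition adjusts an offset's sign along one axis so adding it moves the actor's position toward the destination.
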(fn `GetForwardAimLocation`
  (params (Follower :type "Actor Object Reference") (ForwardAimDistance :type "Float (double-precision)"))
  (returns (FrontLocation :type "Vector Structure"))
  (bind _returnvalue (`ActorComponent.GetOwner` (`Actor.RootComponent` Follower)))
  (return (+ (`Actor.K2_GetActorLocation` _returnvalue) (* (`Actor.GetActorForwardVector` _returnvalue) ForwardAimDistance))))

(fn `SignByPosition`
  (params (VOffset :type "Float (double-precision)") (ActorVPos :type "Float (double-precision)") (DestVPos :type "Float (double-precision)"))
  (returns (FinalOffset :type "Float (double-precision)"))
  (locals (Offset :type "Float (double-precision)"))
  ; We are adding, so we need to account for negatives
  ; if v is negative, negate
  (bind _output_get (set `local.Offset` VOffset))
  (if (< VOffset 0.0)
    (bind _result (`/Engine/EditorBlueprintResources/StandardMacros.NegateFloat` _output_get)
      (:`  `
        (bind _output_get_2 (set `local.Offset` _result)))))
  (if (not (< ActorVPos DestVPos))
    ; Undo negate
    (bind _result_2 (`/Engine/EditorBlueprintResources/StandardMacros.NegateFloat` _output_get_2)
      (:`  `
        (set `local.Offset` _result_2))))
  (return (`local.Offset`)))

(fn `SignedAngle`
  (params (A :type "Vector Structure") (B :type "Vector Structure"))
  (returns (Return :type "Float (double-precision)"))
  (bind (_returnvalue_x _returnvalue_y _returnvalue_z) (`KismetMathLibrary.BreakVector` (`KismetMathLibrary.Cross_VectorVector` A B)))
  (bind _returnvalue (`KismetMathLibrary.Acos` (`KismetMathLibrary.Dot_VectorVector` A B)))
  (if (< _returnvalue_z 0.0)
    (return (* _returnvalue -1.0))
    (else
      (return _returnvalue))))