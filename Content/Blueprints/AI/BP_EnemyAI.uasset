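; Enemy AI pawn that wanders to random reachable points, chases and shoots the first-person character on sight, and is destroyed when damage depletes its health.
; Pawn sensing sets a seen flag and starts pursuit; a retriggerable delay clears it and resumes roaming.
; Each pursuit call spawns one ammo actor with sound, as the looping fire timer is disconnected.
; Reaching the player triggers a gated attack montage, still unassigned.
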(event `self.ReceiveTick`
  (params (DeltaSeconds :type "Float (single-precision)"))
  (if (`self.IsSeeingMouse`)
    (`KismetSystemLibrary.Delay` 1.0)
    (else
      (`KismetSystemLibrary.Delay` 1.0)
      (`self.MoveToRandomLocation`))))

(event `self.PawnSensing.OnSeePawn`
  (params (Pawn :type "Pawn Object Reference"))
  (bind _asbp_first_person_character (cast `/Game/FirstPerson/Blueprints/BP_FirstPersonCharacter` Pawn))
  (`|ExecutionSequence`
    (:`then_0`
      (set `self.IsSeeingMouse` true)
      (`self.FollowPlayer`))
    (:`then_1`
      (`KismetSystemLibrary.RetriggerableDelay` 2.0)
      (set `self.IsSeeingMouse` false)
      (`self.MoveToRandomLocation`))))

(event `FollowPlayer`
  (if (`self.IsSeeingMouse`)
    (`|ExecutionSequence`
      (:`then_0`
        (`|AIMoveTo` self (0.0 0.0 0.0) (stale `self.PawnSensing.OnSeePawn` _asbp_first_person_character) 50.0
          (:`then`
            (`KismetSystemLibrary.RetriggerableDelay` 2.0)
            (`self.MoveToRandomLocation`))
          (:`OnSuccess`
            (if (`self.CanAttack`)
              (set `self.CanAttack` false)
              ; need to set animation montage of attack
              (bind _returnvalue (`self.PlayAnimMontage` null))
              (`KismetSystemLibrary.Delay` _returnvalue)
              (set `self.CanAttack` true)))))
      (:`then_1`
        (`self.OnFire`)))
    (else
      (set `self.IsSeeingMouse` false)
      (`self.OnStopFire`))))

(event `OnStopFire`
  ; StopFire
  (`KismetSystemLibrary.K2_ClearAndInvalidateTimerHandle` (`self.TimerHandle`)))

(event `OnFire`
  ; Fire
  (`GameplayStatics.PlaySoundAtLocation` "/Game/Game_Item/Drop/Cue/Cue_iquidSplashPotio25_Cue_Cue.Cue_iquidSplashPotio25_Cue_Cue" (`self.K2_GetActorLocation`) (struct) 0.5 1.0 0.0 null null null null)
  (`|SpawnActorFromClass` "/Game/Blueprints/Weapons/BP_EnemyAmmo.BP_EnemyAmmo_C" (`self.GetTransform`) "Undefined" "MultiplyWithRoot" (`self.GetOwner`) null))

(event `MoveToRandomLocation`
  (if (not (`self.IsSeeingMouse`))
    (`KismetSystemLibrary.Delay` (`KismetMathLibrary.RandomFloatInRange` 2.0 5.0))
    (`|AIMoveTo` self (`NavigationSystemV1.K2_GetRandomReachablePointInRadius` (`self.K2_GetActorLocation`) 1000.0 null null) null)))

(event `self.ReceiveAnyDamage`
  (params (Damage :type "Float (single-precision)") (DamageType :type "DamageType Object Reference") (InstigatedBy :type "Controller Object Reference") (DamageCauser :type "Actor Object Reference"))
  ; Damage
  (bind _output_get (set `self.Health` (- (`self.Health`) Damage)))
  ;; Check to see if health is below 0
  (if (<= _output_get 0.0)
    (`self.K2_DestroyActor`)))

(fn `UserConstructionScript`)